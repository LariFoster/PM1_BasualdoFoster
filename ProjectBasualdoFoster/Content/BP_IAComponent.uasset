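; AI helper component that handles damage forwarding and colored blood effects.
; IADamaged applies damage to a supplied health component, then fires the OnDamage call.
; CreateOwnDynamicMat builds and stores a dynamic instance of M_Blood.
; SpawnParticles spawns NS_Blood without auto-destroy, passes it that shared instance and sets its BloodColor, so each call recolors every effect using it.
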(fn IADamaged
  (params (myHealthComp :type BP%20Health%20Component%20Object%20Reference) (damage :type Float%20%28double-precision%29))
  (Default|TakeDamage myHealthComp damage)
  (Default|CallOnDamage))

(fn CreateOwnDynamicMat
  (bind _returnvalue (Rendering|Material|CreateDynamicMaterialInstance "/Game/Particles/M_Blood.M_Blood" "None" "None" :!class /Script/Engine.KismetMaterialLibrary))
  (bind _output_get (Variables|Default|SetparticleMat _returnvalue))
  (return _output_get))

(fn SpawnParticles
  (params (Location :type Vector) (Value :type Linear%20Color%20Structure))
  (bind _returnvalue (Niagara|SpawnSystematLocation "/Game/Particles/NS_Blood.NS_Blood" Location "0, 0, 0" "1.000000,1.000000,1.000000" false))
  (Class|NiagaraComponent|SetVariableMaterial _returnvalue "DynamicMaterial" (Variables|Default|GetparticleMat))
  (Rendering|Material|SetVectorParameterValue (Variables|Default|GetparticleMat) "BloodColor" Value :!class /Script/Engine.MaterialInstanceDynamic))
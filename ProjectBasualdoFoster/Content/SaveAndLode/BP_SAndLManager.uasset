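; Save and load manager that stores the player pawn's transform and current level name in a BP_Save slot named by SaveName.
; SaveGame updates the existing save or creates a new one, then writes it to the slot.
; LoadGame opens the saved level, or MAP_FirstPerson when no save exists.
; The saved transform is set immediately after the OpenLevel call, without waiting for the new level to load.
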(event Custom|Save%20Game
  (bind _returnvalue (Game|Player|GetPlayerPawn 0))
  (bind _savename (Variables|Default|GetSaveName))
  (bind _savename_2 (Variables|Default|GetSaveName))
  (bind _returnvalue_2 (Transformation|GetActorTransform _returnvalue))
  (bind _returnvalue_3 (SaveGame|DoesSaveGameExist _savename_2))
  (if _returnvalue_3
    (bind _returnvalue_4 (SaveGame|LoadGamefromSlot _savename_2))
    (bind _asbp_save (Utilities|Casting|CastToBP_Save _returnvalue_4))
    (Variables|/Game/SaveAndLode/BP_Save.BP_Save_C|SetPlayerPos _asbp_save _returnvalue_2)
    (bind _returnvalue_5 (Game|GetCurrentLevelName true))
    (Variables|/Game/SaveAndLode/BP_Save.BP_Save_C|SetLevel _asbp_save _returnvalue_5)
    (SaveGame|SaveGametoSlot _asbp_save _savename)
    (else
      (bind _returnvalue_6 (SaveGame|CreateSaveGameObject "/Game/SaveAndLode/BP_Save.BP_Save_C"))
      (Variables|/Game/SaveAndLode/BP_Save.BP_Save_C|SetPlayerPos _returnvalue_6 _returnvalue_2)
      (bind _returnvalue_7 (Game|GetCurrentLevelName true))
      (Variables|/Game/SaveAndLode/BP_Save.BP_Save_C|SetLevel _returnvalue_6 _returnvalue_7)
      (SaveGame|SaveGametoSlot _returnvalue_6 _savename))))

(event Custom|Load%20Game
  (bind _returnvalue (SaveGame|DoesSaveGameExist (Variables|Default|GetSaveName)))
  (if _returnvalue
    (bind _returnvalue_2 (SaveGame|LoadGamefromSlot (Variables|Default|GetSaveName)))
    (bind _asbp_save (Utilities|Casting|CastToBP_Save _returnvalue_2))
    (Game|OpenLevel(byName) (Utilities|String|StringToName (Variables|/Game/SaveAndLode/BP_Save.BP_Save_C|GetLevel _asbp_save)))
    (bind _output_get (Variables|Default|SetPlayerPos (Variables|/Game/SaveAndLode/BP_Save.BP_Save_C|GetPlayerPos _asbp_save)))
    (Transformation|SetActorTransform (Game|Player|GetPlayerPawn 0) _output_get)
    (else
      (Game|OpenLevel(byName) "MAP_FirstPerson"))))
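; BP_Save is a save data object that holds the player's position, health and level name, plus colour blind severity settings.
; Simple setters store the player values, and LoadSettingValues returns the colour blind severity info.
; The IsSaved checks infer saved state by comparing against sentinel values rather than flags, so full health or a position at the origin reads as unsaved.
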(fn SetLastPlayerPos
  (params (LastPlayerPos :type Vector))
  (Variables|Default|SetPlayerPos LastPlayerPos))

(fn SetPlayerHealth
  (params (PlayerHealth :type Float%20%28double-precision%29))
  (Variables|Default|SetPlayerHealth PlayerHealth))

(fn SetLastLevelName
  (params (LastLevel :type Name))
  (Variables|Default|SetLevel LastLevel))

(fn IsPlayerPosSaved
  (return (not (Class|KismetMathLibrary|EqualExactlyVectorVector (Variables|Default|GetPlayerPos) "0, 0, 0"))))

(fn IsLevelSaved
  (return (!= (Variables|Default|GetLevel) "")))

(fn IsHealthSaved
  (return (not (== (Variables|Default|GetPlayerHealth) 1e+02))))

(fn LoadSettingValues
  (return (Variables|Default|GetColorBlindSeverityInfo)))
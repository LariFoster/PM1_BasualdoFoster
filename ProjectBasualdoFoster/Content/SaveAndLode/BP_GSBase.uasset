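; BP_GSBase, likely a Game State, saves and loads player position, health and current level through a BP_Save object in one slot.
; SaveGame writes a fresh save object from the pawn and PlayerRef.
; LoadGame applies saved position and health before opening the saved level or MAP_FirstPerson, and each missing position or health value halts the chain.
; Without a save, it creates one first; a looping timer is unconnected.
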(event Custom|SaveGame
  (bind _returnvalue (SaveGame|CreateSaveGameObject "/Game/SaveAndLode/BP_Save.BP_Save_C"))
  (bind _output_get (Variables|Default|SetSaveGameRef _returnvalue))
  (Default|SetLastPlayerPos _output_get (Transformation|GetActorLocation (Game|Player|GetPlayerPawn 0)))
  (bind _returnvalue_2 (Game|GetCurrentLevelName true))
  (Default|SetLastLevelName _output_get (Utilities|String|StringToName _returnvalue_2))
  (Default|SetPlayerHealth _output_get (Variables|/Game/FirstPerson/Blueprints/BP_FirstPersonCharacter.BP_FirstPersonCharacter_C|GetHealth (Variables|Default|GetPlayerRef)))
  (SaveGame|SaveGametoSlot (Variables|Default|GetSaveGameRef) (Variables|Default|GetSaveSlot1)))

(event Custom|LoadGame
  (bind _returnvalue (SaveGame|DoesSaveGameExist (Variables|Default|GetSaveSlot1)))
  (if _returnvalue
    (bind _returnvalue_2 (SaveGame|LoadGamefromSlot (Variables|Default|GetSaveSlot1)))
    (bind _asbp_save (Utilities|Casting|CastToBP_Save _returnvalue_2))
    (bind _output_get (Variables|Default|SetSaveGameRef _asbp_save))
    (if (Default|IsPlayerPosSaved _output_get)
      (Transformation|SetActorLocation (Game|Player|GetPlayerPawn 0) (Variables|/Game/SaveAndLode/BP_Save.BP_Save_C|GetPlayerPos (Variables|Default|GetSaveGameRef)) false false)
      (bind _output_get_2 (Variables|Default|SetSaveGameRef _asbp_save))
      (if (Default|IsHealthSaved _output_get_2)
        (bind _output_get_3 (Variables|Default|SetPlayerRef (Variables|Default|GetPlayerRef)))
        (Variables|/Game/FirstPerson/Blueprints/BP_FirstPersonCharacter.BP_FirstPersonCharacter_C|SetHealth _output_get_3 (Variables|/Game/SaveAndLode/BP_Save.BP_Save_C|GetPlayerHealth (Variables|Default|GetSaveGameRef)))
        (bind _output_get_4 (Variables|Default|SetSaveGameRef _asbp_save))
        (if (Default|IsLevelSaved _output_get_4) :!label _label
          (Game|OpenLevel(byName) (Variables|/Game/SaveAndLode/BP_Save.BP_Save_C|GetLevel (Variables|Default|GetSaveGameRef)))
          (else
            (Game|OpenLevel(byObjectReference) "/Game/FirstPerson/Maps/MAP_FirstPerson.MAP_FirstPerson")))))
    (else
      (bind _returnvalue_3 (SaveGame|CreateSaveGameObject "/Game/SaveAndLode/BP_Save.BP_Save_C"))
      (bind _output_get_5 (Variables|Default|SetSaveGameRef _returnvalue_3))
      (SaveGame|SaveGametoSlot _output_get_5 (Variables|Default|GetSaveSlot1))
      (goto _label))))

(fn ConstructionScript)
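; BP_SLManager is a simple save/load manager that stores the player pawn's transform in a BP_SaveG slot.
; On BeginPlay it loads the slot and moves the pawn to the saved transform, or creates the save from the current transform.
; The L key writes the pawn's transform to the slot.
; The M key applies the cached transform to the manager actor itself, not the pawn, without rereading the slot.
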(event EventBeginPlay
  (bind _returnvalue (SaveGame|DoesSaveGameExist (Variables|Default|GetSaveGameName)))
  (if _returnvalue
    (bind _returnvalue_2 (SaveGame|LoadGamefromSlot (Variables|Default|GetSaveGameName)))
    (bind _asbp_save_g (Utilities|Casting|CastToBP_SaveG _returnvalue_2))
    (Variables|Default|SetBP%20SaveG _asbp_save_g)
    (Transformation|SetActorTransform (Game|Player|GetPlayerPawn 0) (Variables|/Game/SaveAndLode/SimpleSave/BP_SaveG.BP_SaveG_C|GetPlayerPos _asbp_save_g))
    (else
      (bind _returnvalue_3 (SaveGame|CreateSaveGameObject "/Game/SaveAndLode/SimpleSave/BP_SaveG.BP_SaveG_C"))
      (Variables|/Game/SaveAndLode/SimpleSave/BP_SaveG.BP_SaveG_C|SetPlayerPos _returnvalue_3 (Transformation|GetActorTransform (Game|Player|GetPlayerPawn 0)))
      (SaveGame|SaveGametoSlot _returnvalue_3 (Variables|Default|GetSaveGameName))
      (Variables|Default|SetBP%20SaveG _returnvalue_3))))

(event Input|KeyboardEvents|L
  (params (Key :type Key%20Structure :default "None"))
  (bind _bp_saveg (Variables|Default|GetBP%20SaveG))
  (:Pressed
    (bind _returnvalue (SaveGame|DoesSaveGameExist (Variables|Default|GetSaveGameName)))
    (if _returnvalue
      (Variables|/Game/SaveAndLode/SimpleSave/BP_SaveG.BP_SaveG_C|SetPlayerPos _bp_saveg (Transformation|GetActorTransform (Game|Player|GetPlayerPawn 0)))
      (SaveGame|SaveGametoSlot _bp_saveg (Variables|Default|GetSaveGameName))
      (Development|PrintString "GAME SAVED"))))

(event Input|KeyboardEvents|M
  (params (Key :type Key%20Structure :default "None"))
  (:Pressed
    (bind _returnvalue (SaveGame|DoesSaveGameExist (Variables|Default|GetSaveGameName)))
    (if _returnvalue
      (Transformation|SetActorTransform (Variables|/Game/SaveAndLode/SimpleSave/BP_SaveG.BP_SaveG_C|GetPlayerPos (Variables|Default|GetBP%20SaveG)))
      (Development|PrintString "GAME LOADED"))))

(fn ConstructionScript)